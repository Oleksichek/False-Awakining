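; Base quest actor that reports its success or failure to a quest manager.
; Initialize stores the manager and, if given a valid event, keeps it as the active event and flags the quest as event-locked.
; StartQuest is an empty hook, while the event completed and failed handlers call EndQuest or FailQuest, which notify the manager and destroy the actor.
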(event Custom|StartQuest)

(event Custom|OnEventCompleted
  (CallFunction|EndQuest))

(event Custom|OnEventFailed
  (CallFunction|FailQuest))

(fn ConstructionScript)

(fn Initialize
  (params (Manager :type BP%20Quest%20Manager%20Object%20Reference) (Event :type BP%20Event%20Base%20Object%20Reference))
  (Variables|Default|SetQuestManager Manager)
  (Utilities|IsValid Event
    (:Is%20Valid
      (Variables|Default|SetActiveEvent Event)
      (Variables|Default|SetIsLockedByEvent true))
    (:Is%20Not%20Valid
      (Variables|Default|SetIsLockedByEvent false))))

(fn EndQuest
  (Default|OnQuestCompleted (Variables|Default|GetQuestManager))
  (Actor|DestroyActor))

(fn FailQuest
  (Default|OnQuestFailed (Variables|Default|GetQuestManager))
  (Actor|DestroyActor))