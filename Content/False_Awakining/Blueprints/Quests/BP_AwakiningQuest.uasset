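; Quest actor for the Awakining quest, which completes once the player holds door key 1.
; Each tick, unless the quest is locked by an event, it casts player character 0 to BP_Player and calls EndQuest when DoorKeys contains that key.
; StartQuest only prints the quest name and whether an ActiveEvent is valid.
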(event EventTick
  (params (DeltaSeconds :type Float%20%28single-precision%29))
  (if (not (Variables|Default|GetIsLockedByEvent))
    (bind _asbp_player (Utilities|Casting|CastToBP_Player (Game|GetPlayerCharacter 0)))
    (if (Utilities|Array|ContainsItem (Variables|/Game/FPMovement/Player/Blueprints/BP_Player.BP_Player_C|GetDoorKeys _asbp_player) 1)
      (CallFunction|EndQuest))))

(event EventStartQuest
  (Development|PrintString (Variables|Default|GetQuestName))
  (Development|PrintString (Utilities|String|ToString(Boolean) (Utilities|IsValid (Variables|Default|GetActiveEvent)))))

(fn ConstructionScript
  (|CallParentFunction))