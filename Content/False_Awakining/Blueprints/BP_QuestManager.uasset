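; Quest manager that runs a list of quests in order, spawning each at its own transform and advancing when one completes.
; On BeginPlay it maps randomly picked quest indices to random events from QuestEventMap, though the picked index refers to the accumulating NotUsedQuests array rather than Quests.
; Quests with a mapped event receive it spawned and are started, while others are only initialized.
; Failure, restart and event-binding handlers are empty stubs.
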(event Custom|OnQuestCompleted
  (Variables|Default|SetCurrentQuestIndex (+ (Variables|Default|GetCurrentQuestIndex) 1))
  (CallFunction|StartNextQuest))

(event Custom|OnQuestFailed)

(event EventBeginPlay
  (CallFunction|GenerateRandomEvents)
  (CallFunction|StartNextQuest))

(fn ConstructionScript)

(fn StartNextQuest
  (bind _self self)
  (bind _returnvalue (Game|SpawnActorfromClass (Utilities|Array|Get(acopy) (Variables|Default|GetQuests) (Variables|Default|GetCurrentQuestIndex)) (Transformation|GetActorTransform) "Undefined" "MultiplyWithRoot" 0 0))
  (bind _output_get (Variables|Default|SetCurrentQuest _returnvalue))
  (if (Utilities|Map|Contains (Variables|Default|GetSelectedEventMap) (Variables|Default|GetCurrentQuestIndex))
    (bind _returnvalue_2 (Game|SpawnActorfromClass (.Value (Utilities|Map|Find (Variables|Default|GetSelectedEventMap) (Variables|Default|GetCurrentQuestIndex))) (Transformation|GetActorTransform) "Undefined" "MultiplyWithRoot" 0 0))
    (Default|Initialize _output_get _self _returnvalue_2)
    (Default|StartQuest _output_get)
    (else
      (Default|Initialize _output_get _self))))

(fn RestartLevel)

(fn SelectRandomEvent)

(fn BindQuestEvents())

(fn GenerateRandomEvents
  (for _index (range 0 (- (Variables|Default|GetBaseEventsCount) 1))
    (bind (_quest _index_2) (CallFunction|GetNotUsedQuest))
    (LocalVariables|SetcurrRandomQuest _quest)
    (bind _array_element (Utilities|Array|ForEachLoopwithBreak (Variables|Default|GetQuestEventMap) :!label _label)
      (:LoopBody
        (if (== (.QuestId (Utilities|Struct|BreakS_QuestEvents _array_element)) _index_2)
          (Utilities|Map|Add (Variables|Default|GetSelectedEventMap) _index_2 (.OutItem (Utilities|Array|Random (.Events (Utilities|Struct|BreakS_QuestEvents _array_element)))))
          (Development|PrintString (Utilities|GetClassDisplayName (.OutItem (Utilities|Array|Random (.Events (Utilities|Struct|BreakS_QuestEvents _array_element))))))
          (goto _label Break))))))

(fn GetNotUsedQuest
  (bind _notusedquests (LocalVariables|GetnotUsedQuests))
  (bind (_outitem _outindex) (Utilities|Array|Random _notusedquests))
  (for (_array_element _array_index) (Variables|Default|GetQuests)
    (if (not (Utilities|Map|Contains (Variables|Default|GetSelectedEventMap) _array_index))
      (Utilities|Array|Add _notusedquests _array_element)))
  (return _outitem _outindex))