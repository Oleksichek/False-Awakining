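; BP_SubtitleTrigger is a one-shot trigger volume that shows a subtitle when the player walks into it.
; On box overlap it casts to BP_Player, passes its Subtitle to the player's SubtitleWidget via StartSubtitle, then destroys itself.
; The construction script scales the box from length, thickness and height variables and makes it visible in game only when DevelopmentMode is on.
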(event OnComponentBeginOverlap(Box)
  (params (OverlappedComponent :type Primitive%20Component%20Object%20Reference) (OtherActor :type Actor%20Object%20Reference) (OtherComp :type Primitive%20Component%20Object%20Reference) (OtherBodyIndex :type Integer) (bFromSweep :type Boolean) (SweepResult :type Hit%20Result%20Structure%20%28by%20ref%29))
  ;[0.05098 0.05098 0.05098] Flashlight Flicker function
  (bind _asbp_player (Utilities|Casting|CastToBP_Player OtherActor))
  (Default|StartSubtitle (Variables|/Game/FPMovement/Player/Blueprints/BP_Player.BP_Player_C|GetSubtitleWidget _asbp_player) (Variables|Default|GetSubtitle))
  (Actor|DestroyActor))

(fn ConstructionScript
  (Transformation|SetWorldScale3D (Variables|Default|GetBox) (Math|Vector|MakeVector (Variables|TriggerBoxSettings|GetBox%20Length) (Variables|TriggerBoxSettings|GetBox%20Thickness) (Variables|TriggerBoxSettings|GetBox%20Height)))
  (if (Variables|TriggerGeneralSettings|GetDevelopmentMode?)
    (Development|SetHiddeninGame (Variables|Default|GetBox) false false)
    (else
      (Development|SetHiddeninGame (Variables|Default|GetBox) true false))))